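; BP_SimpleNPC is an NPC that uses the AI Bridge subsystem for transcribed speech and AI responses.
; It listens for subsystem results, ignores request IDs its NpcClient does not own, and adds matching transcriptions to the chat history as user messages.
; Both transcriptions and AI responses fire its own dispatchers, which briefly flash the skeletal mesh with an interact material as visual feedback.
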(event Custom|OnAiResponseReceived_Event
  (Rendering|Material|SetMaterial (Variables|Default|GetSkeletalMesh) 0 "/Game/NPCs/M_Interact.M_Interact")
  (Utilities|FlowControl|Delay 0.2)
  (Rendering|Material|SetMaterial (Variables|Default|GetSkeletalMesh) 0 (Variables|Default|GetBaseMaterial)))

(event Custom|OnTranscriptionReceived_Event
  (Rendering|Material|SetMaterial (Variables|Default|GetSkeletalMesh) 0 "/Game/NPCs/M_Interact.M_Interact")
  (Utilities|FlowControl|Delay 0.2)
  (Rendering|Material|SetMaterial (Variables|Default|GetSkeletalMesh) 0 (Variables|Default|GetBaseMaterial)))

(event Custom|OnTranscriptionComplete_Event
  (params (RequestId :type String) (Message :type String))
  (if (Utilities|Set|Contains (Variables|/Script/AiBridge.NpcClientComponent|GetRequestIds (Variables|Default|GetNpcClient)) RequestId)
    (Class|NpcClientComponent|AddChatMessage (Variables|Default|GetNpcClient) (Utilities|Struct|MakeChatMessage "user" Message))
    (Default|CallOnTranscriptionReceived)))

(event Custom|OnAiResponse_Event
  (params (RequestId :type String) (Message :type String))
  (if (Utilities|Set|Contains (Variables|/Script/AiBridge.NpcClientComponent|GetRequestIds (Variables|Default|GetNpcClient)) RequestId)
    (Default|CallOnAiResponseReceived)))

(event EventBeginPlay
  (Utilities|FlowControl|Sequence
    (:then_0
      (EventDispatchers|BindEventtoOnTranscriptionComplete (Subsystems|GetAiBridgeSubsystem) (delegate Custom|OnTranscriptionComplete_Event)))
    (:then_1
      (EventDispatchers|BindEventtoOnAiResponse (Subsystems|GetAiBridgeSubsystem) (delegate Custom|OnAiResponse_Event)))
    (:then_2
      (Variables|Default|SetBaseMaterial (Rendering|Material|GetMaterial (Variables|Default|GetSkeletalMesh) 0)))
    (:then_3
      (Utilities|FlowControl|Sequence
        (:then_0
          (EventDispatchers|BindEventtoOnAiResponseReceived (delegate Custom|OnAiResponseReceived_Event)))
        (:then_1
          (EventDispatchers|BindEventtoOnTranscriptionReceived (delegate Custom|OnTranscriptionReceived_Event)))))))

(fn ConstructionScript)